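; BP_Wheat is a farm collectable that disappears when collected and respawns after a delay.
; A sphere overlap with BP_TopDownCharacter sets the CanCollect flag and shows a prompt widget, and leaving clears both.
; Pressing E while CanCollect is set hides the actor and disables its collision, then restores both after RespawnTimer.
; The graph grants no item or inventory reward.
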(event OnComponentBeginOverlap(Sphere)
  (params (OverlappedComponent :type Primitive%20Component%20Object%20Reference) (OtherActor :type Actor%20Object%20Reference) (OtherComp :type Primitive%20Component%20Object%20Reference) (OtherBodyIndex :type Integer) (bFromSweep :type Boolean) (SweepResult :type Hit%20Result%20Structure%20%28by%20ref%29))
  ;[0.15 0.15 0.15 0.5] Set actor to hide and respawn.
  (Utilities|Casting|CastToBP_TopDownCharacter OtherActor)
  (Variables|Default|SetCanCollect true)
  (Rendering|SetVisibility (Variables|Default|GetWidget) true false))

(event OnComponentEndOverlap(Sphere)
  (params (OverlappedComponent :type Primitive%20Component%20Object%20Reference) (OtherActor :type Actor%20Object%20Reference) (OtherComp :type Primitive%20Component%20Object%20Reference) (OtherBodyIndex :type Integer))
  ;[0.15 0.15 0.15 0.5] Set actor to hide and respawn.
  (Utilities|Casting|CastToBP_TopDownCharacter OtherActor)
  (Variables|Default|SetCanCollect false)
  (Rendering|SetVisibility (Variables|Default|GetWidget) false false))

(event Input|KeyboardEvents|E
  (params (Key :type Key%20Structure :default "None"))
  ;[0.15 0.15 0.15 0.5] Set actor to hide and respawn.
  (:Pressed
    (if (Variables|Default|GetCanCollect)
      (Rendering|SetActorHiddenInGame true)
      (Collision|SetActorEnableCollision false)
      (Utilities|FlowControl|Delay (Variables|Default|GetRespawnTimer))
      (Rendering|SetActorHiddenInGame false)
      (Collision|SetActorEnableCollision true))))

(fn ConstructionScript)